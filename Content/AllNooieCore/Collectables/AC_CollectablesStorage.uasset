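; Actor component that stores the player's collectable totals for Jiggys, Notes and Health.
; CollectCollectable switches on the collectable name and adds the given amount to the matching counter.
; It then fires the CollectedCollectable event dispatcher with the name and amount so listeners can react to each pickup.
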(fn CollectCollectable
  (params (Name :type Name) (Amount :type Integer))
  (Utilities|FlowControl|Sequence
    (:then_0
      (switch string (Utilities|String|ToString(Name) Name)
        (:Jiggy
          (Variables|Default|SetJiggys (+ (Variables|Default|GetJiggys) Amount)))
        (:Note
          (Variables|Default|SetNotes (+ (Variables|Default|GetNotes) Amount)))
        (:Health
          (Variables|Default|SetHealth (+ (Variables|Default|GetHealth) Amount)))))
    (:then_1
      (Default|CallCollectedCollectable Name Amount))))