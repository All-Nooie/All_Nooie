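; Collectable item actor that the player picks up on touch, passing its name, UI sprite and amount to the character.
; Sphere overlap asks the player through a message whether items can be accepted, then runs Collect once to send the item and play an optional 2D sound.
; Removal goes through a separate animation-named event that simply destroys the actor.
; Sphere hits from anything but the player play a random impact sound at the mesh.
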(event OnComponentBeginOverlap(Sphere)
  (params (OverlappedComponent :type Primitive%20Component%20Object%20Reference) (OtherActor :type Actor%20Object%20Reference) (OtherComp :type Primitive%20Component%20Object%20Reference) (OtherBodyIndex :type Integer) (bFromSweep :type Boolean) (SweepResult :type Hit%20Result%20Structure%20%28by%20ref%29))
  (bind _returnvalue (Game|GetPlayerCharacter 0))
  (if (== OtherActor _returnvalue)
    (bind _accept_items_ (Class|BICollectable|CanPlayerAcceptItems(Message) _returnvalue))
    (if _accept_items_
      (Utilities|FlowControl|DoOnce false
        (:Completed
          (CallFunction|Collect))))))

(event OnComponentHit(Sphere)
  (params (HitComponent :type Primitive%20Component%20Object%20Reference) (OtherActor :type Actor%20Object%20Reference) (OtherComp :type Primitive%20Component%20Object%20Reference) (NormalImpulse :type Vector :default "0, 0, 0") (Hit :type Hit%20Result%20Structure%20%28by%20ref%29))
  (bind _inpactsounds (Variables|Collectable|Sounds|GetInpactSounds))
  (if (not (== OtherActor (Game|GetPlayerCharacter 0)))
    (if (Utilities|Array|IsValidIndex _inpactsounds)
      (Audio|PlaySoundatLocation (.OutItem (Utilities|Array|Random _inpactsounds)) (Transformation|GetWorldLocation (Variables|Default|GetCollectableMesh)) "0, 0, 0" 1.0 1.0 0.0 0 0 0 0))))

(event Custom|RemoveItemFromMapWithAnimation
  (Actor|DestroyActor))

(event Custom|Collect
  (Class|BICollectable|PlayerCollectItem(Message) (Game|GetPlayerCharacter 0) (Variables|Collectable|Data|GetName) (Variables|Collectable|Data|GetUI%20Sprite) (Variables|Collectable|Data|GetAmount))
  (bind _collectsound (Variables|Collectable|Sounds|GetCollectSound)
    (:then
      (Audio|PlaySound2D _collectsound 1.0 1.0 0.0 0 0))
    (:else
      _))
  (CallFunction|RemoveItemfromMapwithAnimation))

(fn ConstructionScript)