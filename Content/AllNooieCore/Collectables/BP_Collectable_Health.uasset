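; Health pickup collectable that the player can collect unless their stored Health equals the cap of five.
; On Collect, it reads Health from the player's AC_CollectablesStorage component, then sends the player a collect-item message with name, sprite and amount.
; It then plays an optional 2D sound and removes itself from the map with an animation.
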(event EventBeginPlay)

(event Collision|EventActorBeginOverlap
  (params (OtherActor :type Actor%20Object%20Reference)))

(event EventTick
  (params (DeltaSeconds :type Float%20%28single-precision%29)))

(event EventCollect
  (if (not (== (Variables|/Game/AllNooieCore/Collectables/AC_CollectablesStorage.AC_CollectablesStorage_C|GetHealth (Actor|GetComponentbyClass (Game|GetPlayerCharacter 0) "/Game/AllNooieCore/Collectables/AC_CollectablesStorage.AC_CollectablesStorage_C")) 5))
    (Class|BICollectable|PlayerCollectItem(Message) (Game|GetPlayerCharacter 0) (Variables|Default|GetName) (Variables|Default|GetUI%20Sprite) (Variables|Default|GetAmount))
    (bind _collectsound (Variables|Default|GetCollectSound)
      (:then
        (Audio|PlaySound2D _collectsound 1.0 1.0 0.0 0 0))
      (:else
        _))
    (CallFunction|RemoveItemfromMapwithAnimation)))

(fn ConstructionScript
  (|CallParentFunction))